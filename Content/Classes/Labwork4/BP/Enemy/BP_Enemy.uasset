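; BP_Enemy is a turret-like enemy that fires BP_EnemyBeam actors and destroys itself when hit.
; A looping timer started on BeginPlay, after a successful player-character cast, drives a FlipFlop that alternates spawns between the mesh's left and right gun sockets.
; Tick uses a DoOnce and FlipFlop to play and reverse a timeline, sweeping the mesh's yaw back and forth.
; The cached player reference is not used for aiming.
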(event `self.ReceiveBeginPlay`
  (bind _asbp_third_person_character_labwork_3 (cast `/Game/Classes/LabWork3/BP_ThirdPersonCharacterLabwork3` (`GameplayStatics.GetPlayerPawn` 0)))
  (set `self.Player` _asbp_third_person_character_labwork_3)
  (`KismetSystemLibrary.K2_SetTimerDelegate` (delegate `FireBeam`) 0.1 true))

(event `FireBeam`
  (bind (_returnvalue_location _returnvalue_rotation) (`KismetMathLibrary.BreakTransform` (`SceneComponent.GetSocketTransform` (`self.StaticMesh`) "R_Gun" "RTS_World")))
  (bind (_returnvalue_location_2 _returnvalue_rotation_2) (`KismetMathLibrary.BreakTransform` (`SceneComponent.GetSocketTransform` (`self.StaticMesh`) "L_Gun" "RTS_World")))
  (`/Engine/EditorBlueprintResources/StandardMacros.FlipFlop`
    (:`A`
      (`|SpawnActorFromClass` "/Game/Classes/Labwork4/BP/Enemy/BP_EnemyBeam.BP_EnemyBeam_C" (`KismetMathLibrary.MakeTransform` _returnvalue_location_2 _returnvalue_rotation_2) "Undefined" "MultiplyWithRoot" null null))
    (:`B`
      (`|SpawnActorFromClass` "/Game/Classes/Labwork4/BP/Enemy/BP_EnemyBeam.BP_EnemyBeam_C" (`KismetMathLibrary.MakeTransform` _returnvalue_location _returnvalue_rotation) "Undefined" "MultiplyWithRoot" null null))))

(event `self.ReceiveTick`
  (params (DeltaSeconds :type "Float (single-precision)"))
  (`/Engine/EditorBlueprintResources/StandardMacros.DoOnce` false :!label _label
    (:`Completed`
      (`/Engine/EditorBlueprintResources/StandardMacros.FlipFlop`
        (:`A`
          (bind (_direction _yrot) (`Timeline|Timeline` :!label _label_2)
            (:`Update`
              (`SceneComponent.K2_SetRelativeRotation` (`self.StaticMesh`) (`KismetMathLibrary.MakeRotator` 0.0 0.0 _yrot) false false))
            (:`Finished`
              (goto _label :!via `Reset`))))
        (:`B`
          (goto _label_2 :!via `Reverse`))))))

(event `/Game/Classes/Labwork4/BP/Interface/BPI_Hit.Hit`
  (`self.K2_DestroyActor`))

(fn `UserConstructionScript`)