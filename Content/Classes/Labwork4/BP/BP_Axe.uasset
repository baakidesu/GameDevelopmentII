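; BP_Axe is a swinging axe hazard that damages the player on contact.
; Tick runs a DoOnce into a FlipFlop that alternately plays and reverses the YRot timeline, which drives mesh pitch and resets the DoOnce when finished, looping the swing.
; BeginPlay caches the player as BP_ThirdPersonCharacterLabwork3.
; Any mesh hit calls that player's DamageFunction, only once because its DoOnce never resets, without checking what was hit.
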(event `self.ReceiveTick`
  (params (DeltaSeconds :type "Float (single-precision)"))
  (`/Engine/EditorBlueprintResources/StandardMacros.DoOnce` false :!label _label
    (:`Completed`
      (`/Engine/EditorBlueprintResources/StandardMacros.FlipFlop`
        (:`A`
          (bind (_direction _yrot) (`Timeline|YRot` :!label _label_2)
            (:`Update`
              (`SceneComponent.K2_SetRelativeRotation` (`self.StaticMesh`) (`KismetMathLibrary.MakeRotator` 180.0 _yrot) false false))
            (:`Finished`
              (goto _label :!via `Reset`))))
        (:`B`
          (goto _label_2 :!via `Reverse`))))))

(event `self.ReceiveBeginPlay`
  (bind _asbp_third_person_character_labwork_3 (cast `/Game/Classes/LabWork3/BP_ThirdPersonCharacterLabwork3` (`GameplayStatics.GetPlayerPawn` 0)))
  (set `self.Player` _asbp_third_person_character_labwork_3))

(event `self.StaticMesh.OnComponentHit`
  (params (HitComponent :type "PrimitiveComponent Object Reference") (OtherActor :type "Actor Object Reference") (OtherComp :type "PrimitiveComponent Object Reference") (NormalImpulse :type "Vector Structure") (Hit :type "HitResult Structure (by ref)"))
  (`/Engine/EditorBlueprintResources/StandardMacros.DoOnce` false
    (:`Completed`
      (`/Game/Classes/LabWork3/BP_ThirdPersonCharacterLabwork3.DamageFunction` (`self.Player`)))))

(fn `UserConstructionScript`)