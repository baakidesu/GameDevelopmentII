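; BP_WallMechanic is a sliceable wall actor that breaks off a physics piece at a hit location.
; The construction script copies the static mesh into a procedural mesh with collision, then destroys the original component.
; HitwithLoc prints the location and slices there along a fixed diagonal normal, capping the cut; the new half simulates physics with physics-only collision.
; A scale-then-destroy timeline is left unconnected.
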(event `/Game/Classes/Labwork4/BP/Interface/BPI_Hit.HitWithLoc`
  (params (Vector :type "Vector Structure"))
  (`KismetSystemLibrary.PrintString` (`KismetStringLibrary.Conv_VectorToString` Vector))
  (bind _outotherhalfprocmesh (`KismetProceduralMeshLibrary.SliceProceduralMesh` (`self.ProceduralMesh`) Vector (1.0 1.0 1.0) true "UseLastSectionForCap" "/Game/Classes/Labwork4/M/M_Wall.M_Wall"))
  (`PrimitiveComponent.SetSimulatePhysics` _outotherhalfprocmesh true)
  (`PrimitiveComponent.SetCollisionEnabled` _outotherhalfprocmesh "PhysicsOnly"))

(fn `UserConstructionScript`
  (`KismetProceduralMeshLibrary.CopyProceduralMeshFromStaticMeshComponent` (`self.StaticMesh`) 0 (`self.ProceduralMesh`) true)
  (`ActorComponent.K2_DestroyComponent` (`self.StaticMesh`)))