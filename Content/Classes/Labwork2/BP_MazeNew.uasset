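; BP_MazeNew manages a timed maze round, showing a WB_Timer widget and finding the exit cell on BeginPlay.
; Tick uses a one-second Delay to count down Minutes and Seconds, calling Lose once both reach zero.
; Win and Lose recolor cell lights green or red and set the condition text; Win has no caller here.
; Lose targets BP_MazeCellNew, while Win and the exit search use BP_MazeCellLabwork3.
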(event `self.ReceiveBeginPlay`
  (bind _returnvalue (`|CreateWidget` "/Game/Classes/Labwork2/WB_Timer.WB_Timer_C"))
  (bind _output_get (set `self.Widget` _returnvalue))
  (`UserWidget.AddToViewport` _output_get 0)
  (bind _outactors (`GameplayStatics.GetAllActorsOfClass` "/Game/Classes/LabWork3/BP_MazeCellLabwork3.BP_MazeCellLabwork3_C"))
  (for _array_element _outactors
    (if (`/Game/Classes/LabWork3/BP_MazeCellLabwork3.IsExit` _array_element)
      (set `self.ExitMazeCell` _array_element))))

(event `self.ReceiveTick`
  (params (DeltaSeconds :type "Float (single-precision)"))
  ;[1 1 1] Timer
  (if (`self.didLose`)
    _
    (elif (and (== (`self.Minutes`) 0) (== (`self.Seconds`) 0))
      (`self.Lose`)
      (set `self.didLose` true)
      (else
        (`KismetSystemLibrary.Delay` 1.0)
        (if (> 1 (`self.Seconds`))
          (set `self.Seconds` 59)
          (`/Engine/EditorBlueprintResources/StandardMacros.DecrementInt` (`self.Minutes`))
          (else
            (`/Engine/EditorBlueprintResources/StandardMacros.DecrementInt` (`self.Seconds`))))))))

(fn `Lose`
  (bind _outactors (`GameplayStatics.GetAllActorsOfClass` "/Game/Classes/Labwork2/BP_MazeCellNew.BP_MazeCellNew_C"))
  (for _array_element _outactors
    (set `/Game/Classes/Labwork2/BP_MazeCellNew.LightColor` (struct :`R` 1.0 :`B` 0.022139 :`A` 1.0) _array_element)
    (set `TextBlock.Text` "You Lost!" (`/Game/Classes/Labwork2/WB_Timer.ConditionText` (`self.Widget`)))))

(fn `UserConstructionScript`)

(fn `Win`
  (bind _outactors (`GameplayStatics.GetAllActorsOfClass` "/Game/Classes/LabWork3/BP_MazeCellLabwork3.BP_MazeCellLabwork3_C"))
  (for _array_element _outactors
    (set `/Game/Classes/LabWork3/BP_MazeCellLabwork3.LightColor` (struct :`R` 0.402957 :`G` 1.0 :`A` 1.0) _array_element)
    (set `TextBlock.Text` "" (`/Game/Classes/Labwork2/WB_Timer.ConditionText` (`self.Widget`)))))