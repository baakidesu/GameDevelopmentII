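; A single maze cell actor that also serves as the maze exit when flagged IsExit.
; The construction script scales the floor to GridSize and adds optional walls and a ceiling as static mesh components sized through SizeToCubeScale.
; BeginPlay adds a point light near the top center, and Tick reapplies its color every frame.
; On exit cells, the player pawn hitting the floor calls Win on the BP_MazeNew found at BeginPlay.
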(event `self.ReceiveBeginPlay`
  (bind _returnvalue (* (`self.WallLength`) 0.5))
  (bind _returnvalue_2 (`AddComponent|NODE_AddPointLightComponent-1` :`RelativeTransform` (`KismetMathLibrary.MakeTransform` (`KismetMathLibrary.MakeVector` _returnvalue _returnvalue (* (`self.WallHeight`) 0.9)))))
  (bind _output_get (set `self.Light` _returnvalue_2))
  (`LightComponent.SetLightColor` _output_get (`self.LightColor`) true)
  (`LightComponent.SetIntensity` _output_get (`self.LightIntensity`))
  (if (`self.IsExit`)
    (set `self.IsExit` true)
    (bind _returnvalue_3 (`GameplayStatics.GetActorOfClass` "/Game/Classes/Labwork2/BP_MazeNew.BP_MazeNew_C"))
    (set `self.Maze` _returnvalue_3)))

(event `self.Floor.OnComponentHit`
  (params (HitComponent :type "PrimitiveComponent Object Reference") (OtherActor :type "Actor Object Reference") (OtherComp :type "PrimitiveComponent Object Reference") (NormalImpulse :type "Vector Structure") (Hit :type "HitResult Structure (by ref)"))
  ;[1 1 1] Exit Hit
  (if (`self.IsExit`)
    (if (== OtherActor (`GameplayStatics.GetPlayerPawn` 0))
      (`/Game/Classes/Labwork2/BP_MazeNew.Win` (`self.Maze`)))))

(event `self.ReceiveTick`
  (params (DeltaSeconds :type "Float (single-precision)"))
  ;[1 1 1] Set Light
  (`LightComponent.SetLightColor` (`self.Light`) (`self.LightColor`) true))

(fn `UserConstructionScript`
  (bind _gridsize (`self.GridSize`))
  (bind _walllength (`self.WallLength`))
  (bind _walllength_2 (`self.WallLength`))
  (set `self.WallLength` _gridsize)
  (set `self.WallThickness` (* _gridsize 0.1))
  (`SceneComponent.SetRelativeScale3D` (`self.Floor`) (`self.SizeToCubeScale` (`KismetMathLibrary.MakeVector` _walllength _walllength (`self.WallThickness`))))
  (if (`self.WestWall`)
    (`AddComponent|NODE_AddStaticMeshComponent-0` :`RelativeTransform` (`KismetMathLibrary.MakeTransform` (0.0 0.0 0.0) (struct) (`self.SizeToCubeScale` (`KismetMathLibrary.MakeVector` (`self.WallLength`) (`self.WallThickness`) (`self.WallHeight`))))))
  (if (`self.SouthWall`)
    (`AddComponent|NODE_AddStaticMeshComponent-1` :`RelativeTransform` (`KismetMathLibrary.MakeTransform` (0.0 0.0 0.0) (struct) (`self.SizeToCubeScale` (`KismetMathLibrary.MakeVector` (`self.WallThickness`) (`self.WallLength`) (`self.WallHeight`))))))
  (if (`self.NorthWall`)
    (`AddComponent|NODE_AddStaticMeshComponent-2` :`RelativeTransform` (`KismetMathLibrary.MakeTransform` (`KismetMathLibrary.MakeVector` (- (`self.WallLength`) (`self.WallThickness`))) (struct) (`self.SizeToCubeScale` (`KismetMathLibrary.MakeVector` (`self.WallThickness`) (`self.WallLength`) (`self.WallHeight`))))))
  (if (`self.EastWall`)
    (`AddComponent|NODE_AddStaticMeshComponent-3` :`RelativeTransform` (`KismetMathLibrary.MakeTransform` (`KismetMathLibrary.MakeVector` 0.0 (- (`self.WallLength`) (`self.WallThickness`))) (struct) (`self.SizeToCubeScale` (`KismetMathLibrary.MakeVector` (`self.WallLength`) (`self.WallThickness`) (`self.WallHeight`))))))
  (if (`self.Ceiling`)
    (`AddComponent|NODE_AddStaticMeshComponent-4` :`RelativeTransform` (`KismetMathLibrary.MakeTransform` (`KismetMathLibrary.MakeVector` 0.0 0.0 (`self.WallHeight`)) (struct) (`self.SizeToCubeScale` (`KismetMathLibrary.MakeVector` _walllength_2 _walllength_2 (`self.WallThickness`))))))
  (if (> (`self.LightIntensity`) 0.0)
    _))