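; BP_Key is a collectible key actor that the player picks up by interacting with it.
; On BeginPlay it caches the BP_ThirdPersonCharacterLabwork3 player and creates a dynamic instance of M_Key on the Key component, tinted with its KeyColor.
; Interact adds the key's KeyIndex to the player's Keys collection and then destroys the actor.
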(event `self.ReceiveBeginPlay`
  (bind _asbp_third_person_character_labwork_3 (cast `/Game/Classes/LabWork3/BP_ThirdPersonCharacterLabwork3` (`GameplayStatics.GetPlayerCharacter` 0)))
  (set `self.Player` _asbp_third_person_character_labwork_3)
  (bind _returnvalue (`PrimitiveComponent.CreateDynamicMaterialInstance` (`self.Key`) 0 "/Game/Classes/LabWork3/M_Key.M_Key" "None"))
  (`MaterialInstanceDynamic.SetVectorParameterValue` _returnvalue "Color" (`self.KeyColor`)))

(event `/Game/Classes/LabWork3/BPI_Interact.Interact`
  (`KismetArrayLibrary.Array_Add` (`/Game/Classes/LabWork3/BP_ThirdPersonCharacterLabwork3.Keys` (`self.Player`)) (`self.KeyIndex`))
  (`self.K2_DestroyActor`))

(fn `UserConstructionScript`)