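; Maze cell actor that forms one tile of the maze and can hold gold or serve as the exit.
; The construction script scales the floor from GridSize and adds optional walls and ceiling as scaled static meshes.
; BeginPlay optionally spawns BP_Gold with a weighted random Condition and adds a point light, whose color and intensity Tick reapplies.
; Exit cells find the maze controller and call its Win when the player pawn overlaps the Box.
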(event `self.ReceiveBeginPlay`
  (bind _returnvalue (* (`self.WallLength`) 0.5))
  (`self.CreateGoldMacro`)
  (bind _returnvalue_2 (`AddComponent|NODE_AddPointLightComponent-1` :`RelativeTransform` (`KismetMathLibrary.MakeTransform` (`KismetMathLibrary.MakeVector` _returnvalue _returnvalue (* (`self.WallHeight`) 0.9)))))
  (bind _output_get (set `self.Light` _returnvalue_2))
  (`LightComponent.SetLightColor` _output_get (`self.LightColor`) true)
  (`LightComponent.SetIntensity` _output_get (`self.LightIntensity`))
  (if (`self.IsExit`)
    (set `self.IsExit` true)
    (bind _returnvalue_3 (`GameplayStatics.GetActorOfClass` "/Game/Classes/LabWork3/BP_MazeControllerLabwork3.BP_MazeControllerLabwork3_C"))
    (set `self.Maze` _returnvalue_3)))

(event `self.Box.OnComponentBeginOverlap`
  (params (OverlappedComponent :type "PrimitiveComponent Object Reference") (OtherActor :type "Actor Object Reference") (OtherComp :type "PrimitiveComponent Object Reference") (OtherBodyIndex :type Integer) (bFromSweep :type Boolean) (SweepResult :type "HitResult Structure (by ref)"))
  ;[1 1 1] Exit Hit
  (if (`self.IsExit`)
    (if (== OtherActor (`GameplayStatics.GetPlayerPawn` 0))
      (`/Game/Classes/LabWork3/BP_MazeControllerLabwork3.Win` (`self.Maze`)))))

(event `self.ReceiveTick`
  (params (DeltaSeconds :type "Float (single-precision)"))
  ;[1 1 1] Set Light
  (`LightComponent.SetLightColor` (`self.Light`) (`self.LightColor`) true)
  (`LightComponent.SetIntensity` (`self.Light`) (`self.LightIntensity`)))

(fn `CreateGold`
  (params (condition :type Integer))
  (bind _returnvalue (`|SpawnActorFromClass` "/Game/Classes/LabWork3/BP_Gold.BP_Gold_C" (`KismetMathLibrary.MakeTransform` (+ (`self.K2_GetActorLocation`) (100.0 100.0 100.0))) "Undefined" "MultiplyWithRoot" null 0 null))
  (set `/Game/Classes/LabWork3/BP_Gold.condition` condition _returnvalue))

(fn `UserConstructionScript`
  (`self.ScaleSettings`)
  (`self.CreateWalls`))