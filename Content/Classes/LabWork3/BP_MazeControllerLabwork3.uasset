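; Maze game controller that runs a countdown, hazards and lighting, with win and lose feedback.
; BeginPlay caches the player, creates the timer widget, and gathers maze cells as lights, noting the exit cell.
; Tick uses Delays as pacing for the countdown, periodic beams spawned above the player, and random light intensity changes.
; Timeout calls Lose; Lose and Win recolor cell lights and set widget text, though Win is not called here.
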(event `self.ReceiveBeginPlay`
  ;[0.7939 0.2708 1] Construct
  (bind _asbp_third_person_character_labwork_3 (cast `/Game/Classes/LabWork3/BP_ThirdPersonCharacterLabwork3` (`GameplayStatics.GetPlayerPawn` 0)))
  (set `self.Player` _asbp_third_person_character_labwork_3)
  (bind _returnvalue (`|CreateWidget` "/Game/Classes/LabWork3/WB_TimerWeek4.WB_TimerWeek4_C"))
  (bind _output_get (set `self.Widget` _returnvalue))
  (`UserWidget.AddToViewport` _output_get 0)
  (bind _outactors (`GameplayStatics.GetAllActorsOfClass` "/Game/Classes/LabWork3/BP_MazeCellLabwork3.BP_MazeCellLabwork3_C"))
  (for _array_element _outactors
    (if (`/Game/Classes/LabWork3/BP_MazeCellLabwork3.IsExit` _array_element)
      (set `self.ExitMazeCell` _array_element)))
  (bind _outactors_2 (`GameplayStatics.GetAllActorsOfClass` "/Game/Classes/LabWork3/BP_MazeCellLabwork3.BP_MazeCellLabwork3_C"))
  (set `self.Lights` _outactors_2))

(event `self.ReceiveTick`
  (params (DeltaSeconds :type "Float (single-precision)"))
  (bind _returnvalue (`self.K2_GetActorLocation` (`self.Player`)))
  (`|ExecutionSequence`
    (:`then_0`
      ;[1 0.3504 0.687] Timer
      (if (`self.didLose`)
        _
        (elif (and (== (`self.Minutes`) 0) (== (`self.Seconds`) 0))
          (`self.Lose`)
          (set `self.didLose` true)
          (else
            (`KismetSystemLibrary.Delay` 1.0)
            (if (> 1 (`self.Seconds`))
              (set `self.Seconds` 59)
              (`/Engine/EditorBlueprintResources/StandardMacros.DecrementInt` (`self.Minutes`))
              (else
                (bind _result (`/Engine/EditorBlueprintResources/StandardMacros.DecrementInt` (`self.Seconds`))
                  (:`  `
                    (if (== (mod _result 5) 0)
                      ;[1 0.02217 0.1761] Shoot Player
                      (bind _output_get (set `self.TransformLoc` (+ _returnvalue (0.0 0.0 250.0))))
                      (`|SpawnActorFromClass` "/Game/Classes/Labwork4andMidterm/BP/BP_PawnBeam.BP_PawnBeam_C" (`KismetMathLibrary.MakeTransform` _output_get (`KismetMathLibrary.FindLookAtRotation` (`self.TransformLoc`) _returnvalue)) "Undefined" "MultiplyWithRoot" null null))))))))))
    (:`then_1`
      ;[1 0.9503 0.07605] Change Light Intensity
      (if (not (`self.didLose`))
        (`KismetSystemLibrary.Delay` 0.5)
        (set `self.Light Intensity` (`KismetArrayLibrary.Array_Random` (`self.LightVolumes`)))
        (for _array_element (`self.Lights`)
          (set `/Game/Classes/LabWork3/BP_MazeCellLabwork3.LightIntensity` (`self.Light Intensity`) _array_element))))))

(fn `Lose`
  (for _array_element (`self.Lights`)
    (set `/Game/Classes/LabWork3/BP_MazeCellLabwork3.LightColor` (struct :`R` 1.0 :`B` 0.069467 :`A` 1.0) _array_element)
    (set `TextBlock.Text` "You Lost!" (`/Game/Classes/LabWork3/WB_TimerWeek4.ConditionText` (`self.Widget`)))))

(fn `UserConstructionScript`)

(fn `Win`
  (for _array_element (`self.Lights`)
    (set `/Game/Classes/LabWork3/BP_MazeCellLabwork3.LightColor` (struct :`R` 0.346008 :`G` 1.0 :`B` 0.085258 :`A` 1.0) _array_element)
    (set `TextBlock.Text` "Well Done!" (`/Game/Classes/LabWork3/WB_TimerWeek4.ConditionText` (`self.Widget`)))))