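; Gold pickup actor that adds a random amount of gold to the player character when interacted with.
; The construction script rolls the amount from 1 to 3.
; After a short BeginPlay delay, it caches the lab character reference and shows as many of its three components as the rolled amount.
; Interact adds that amount to the character's Gold and destroys the actor.
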(event `self.ReceiveBeginPlay`
  (`KismetSystemLibrary.Delay` 0.2) ; Construct Delay
  (bind _asbp_third_person_character_labwork_3 (cast `/Game/Classes/LabWork3/BP_ThirdPersonCharacterLabwork3` (`GameplayStatics.GetPlayerCharacter` 0))
    (:`then`
      (set `self.As BP Third Person Character Labwork 3` _asbp_third_person_character_labwork_3)
      (switch `int` (`self.condition`)
        (:`Default`
          (`self.Visibility` false))
        (:`1`
          (`self.Visibility` true))
        (:`2`
          (`self.Visibility` true true))
        (:`3`
          (`self.Visibility` true true true))))
    (:`CastFailed`
      (`KismetSystemLibrary.PrintString` "bozuk"))))

(event `/Game/Classes/LabWork3/BP_Interact.Interact`
  (bind _as_bp_third_person_character_labwork_3 (`self.As BP Third Person Character Labwork 3`))
  (set `/Game/Classes/LabWork3/BP_ThirdPersonCharacterLabwork3.Gold` (+ (`/Game/Classes/LabWork3/BP_ThirdPersonCharacterLabwork3.Gold` _as_bp_third_person_character_labwork_3) (`self.condition`)) _as_bp_third_person_character_labwork_3)
  (`self.K2_DestroyActor`))

(fn `UserConstructionScript`
  (set `self.condition` (`KismetMathLibrary.RandomIntegerInRange` 1 3)))

(fn `Visibility`
  (params (`1` :type Boolean) (`2` :type Boolean) (`3` :type Boolean))
  (`SceneComponent.SetVisibility` (`self.1`) `1` false)
  (`SceneComponent.SetVisibility` (`self.2`) `2` false)
  (`SceneComponent.SetVisibility` (`self.3`) `3` false))