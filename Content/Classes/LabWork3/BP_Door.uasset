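; BP_Door is a locked door actor for LabWork3 that the player opens with a matching key.
; On BeginPlay it caches the third-person lab character and tints its cube with a dynamic M_Key material using DoorColor.
; Interact searches the player's Keys for DoorIndex, destroying the door when found and printing a missing-key message otherwise.
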(event `self.ReceiveBeginPlay`
  (bind _asbp_third_person_character_labwork_3 (cast `/Game/Classes/LabWork3/BP_ThirdPersonCharacterLabwork3` (`GameplayStatics.GetPlayerCharacter` 0)))
  (set `self.Player` _asbp_third_person_character_labwork_3)
  (bind _returnvalue (`PrimitiveComponent.CreateDynamicMaterialInstance` (`self.Cube`) 0 "/Game/Classes/LabWork3/M_Key.M_Key" "None"))
  (`MaterialInstanceDynamic.SetVectorParameterValue` _returnvalue "Color" (`self.DoorColor`)))

(event `/Game/Classes/LabWork3/BPI_Interact.Interact`
  (if (not (== (`KismetArrayLibrary.Array_Find` (`/Game/Classes/LabWork3/BP_ThirdPersonCharacterLabwork3.Keys` (`self.Player`)) (`self.DoorIndex`)) -1))
    (`self.K2_DestroyActor`)
    (else
      (`KismetSystemLibrary.PrintString` "Key Not Found!!" true true (struct :`R` 1.0 :`B` 0.043499 :`A` 1.0)))))

(fn `UserConstructionScript`)