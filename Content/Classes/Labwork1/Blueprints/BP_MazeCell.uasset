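; BP_MazeCell is a single maze cell with North, South, East and West walls, each shown or hidden by its own flag.
; The Construction Script passes every wall and flag to SetVisibilityOfWalls, which sets visibility and rescales the wall vertically by the shared WallHeight.
; That helper also prints WallHeight on each call, and BeginPlay does nothing.
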(event `self.ReceiveBeginPlay`)

(fn `Set Visibility Of Walls`
  (params (Wall :type "SceneComponent Object Reference") (WallVisibility :type Boolean))
  (`KismetSystemLibrary.PrintString` (`KismetStringLibrary.Conv_DoubleToString` (`self._wallHeight`)))
  (`SceneComponent.SetVisibility` Wall WallVisibility false)
  (`SceneComponent.SetRelativeScale3D` Wall (`KismetMathLibrary.MakeVector` 0.0725 1.0 (`self._wallHeight`))))

(fn `UserConstructionScript`
  (`self.Set Visibility Of Walls` (`self.West`) (`self.WestWall`))
  (`self.Set Visibility Of Walls` (`self.East`) (`self.EastWall`))
  (`self.Set Visibility Of Walls` (`self.North`) (`self.NorthWall`))
  (`self.Set Visibility Of Walls` (`self.South`) (`self.SouthWall`)))