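; BP_Maze is a maze base that arranges BP_MazeCell actors already in the level into a grid on a floor slab.
; The construction script scales the Cube by the converted GrizSize and derives wall thickness from it.
; A fixed 7×7 nested loop positions cells at 100-unit spacing from the slab's corner and passes them wall thickness and height.
; It spawns no cells, and BeginPlay is empty.
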(event `self.ReceiveBeginPlay`)

(fn `UserConstructionScript`
  (bind (_returnvalue_x _returnvalue_y) (`KismetMathLibrary.BreakVector` (`self.K2_GetActorLocation`)))
  (bind (_relativescale3d_x _relativescale3d_y) (`KismetMathLibrary.BreakVector` (`SceneComponent.RelativeScale3D` (`self.Cube`))))
  (bind _output_get (set `self.grizSize` (* (`self.grizSize`) 0.01)))
  (set `self.wallThickness` (/ _output_get 10.0))
  (`SceneComponent.SetRelativeScale3D` (`self.Cube`) (`KismetMathLibrary.MakeVector` _output_get _output_get 0.2))
  (bind _outactors (`GameplayStatics.GetAllActorsOfClass` "/Game/Classes/Labwork1/Blueprints/BP_MazeCell.BP_MazeCell_C"))
  (for _index (range 1 8)
    (for _index_2 (range 1 8)
      (`/Engine/EditorBlueprintResources/StandardMacros.IncrementInt` (`self.index`)
        (:`  `
          (bind _output (`|GetArrayItem` _outactors (`self.index`)))
          (`self.K2_SetActorLocation` _output (`KismetMathLibrary.MakeVector` (+ (* (`KismetMathLibrary.Conv_IntToDouble` _index) 100.0) (* _relativescale3d_x -50.0) _returnvalue_x -50.0) (+ _returnvalue_y (* _relativescale3d_y -50.0) (* (`KismetMathLibrary.Conv_IntToDouble` _index_2) 100.0) -50.0)) false false)
          (set `/Game/Classes/Labwork1/Blueprints/BP_MazeCell._wallThickness` (`self.wallThickness`) _output)
          (set `/Game/Classes/Labwork1/Blueprints/BP_MazeCell._wallHeight` (* (`self.wallHeight`) 0.01) _output))))))