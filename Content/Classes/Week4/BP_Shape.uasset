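; BP_Shape is an interactable sphere actor that toggles its material whenever it receives the Interact event.
; Interact prints a debug string, flips the InteractState boolean, and swaps the Sphere between M_Black when on and BasicShapeMaterial when off.
; GetInteractState returns the current toggle value, while BeginPlay, Tick, overlap and construction logic are empty.
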(event `/Game/Classes/Week4/I_Interact.Interact`
  (bind _sphere (`self.Sphere`))
  (`KismetSystemLibrary.PrintString` "za")
  (if (`self.InteractState`)
    (set `self.InteractState` false)
    (`PrimitiveComponent.SetMaterial` _sphere 0 "/Engine/BasicShapes/BasicShapeMaterial.BasicShapeMaterial")
    (else
      (set `self.InteractState` true)
      (`PrimitiveComponent.SetMaterial` _sphere 0 "/Game/Classes/Labwork1/Blueprints/M_Black.M_Black"))))

(fn `GetInteractState`
  (returns (NewParam :type Boolean))
  (return (`self.InteractState`)))

(fn `UserConstructionScript`)