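; BP_Enemy1 is an enemy actor that swings its static mesh in yaw and destroys itself on any Hit event.
; Tick drives a DoOnce and FlipFlop that alternately play and reverse a timeline, resetting on finish for continuous back-and-forth rotation.
; BeginPlay caches the player character, but nothing here uses it.
; Beam spawning from alternating gun sockets and its repeating timer are disconnected, and FireBeam is empty, so it never fires.
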(event `self.ReceiveBeginPlay`
  (bind _asbp_third_person_character_labwork_3 (cast `/Game/Classes/LabWork3/BP_ThirdPersonCharacterLabwork3` (`GameplayStatics.GetPlayerPawn` 0)))
  (set `self.Player` _asbp_third_person_character_labwork_3))

(event `FireBeam`)

(event `self.ReceiveTick`
  (params (DeltaSeconds :type "Float (single-precision)"))
  (`/Engine/EditorBlueprintResources/StandardMacros.DoOnce` false :!label _label
    (:`Completed`
      (`/Engine/EditorBlueprintResources/StandardMacros.FlipFlop`
        (:`A`
          (bind (_direction _yrot) (`Timeline|Timeline` :!label _label_2)
            (:`Update`
              (`SceneComponent.K2_SetRelativeRotation` (`self.StaticMesh`) (`KismetMathLibrary.MakeRotator` 0.0 0.0 _yrot) false false))
            (:`Finished`
              (goto _label :!via `Reset`))))
        (:`B`
          (goto _label_2 :!via `Reverse`))))))

(event `self.Hit`
  (`self.K2_DestroyActor`))

(fn `UserConstructionScript`)