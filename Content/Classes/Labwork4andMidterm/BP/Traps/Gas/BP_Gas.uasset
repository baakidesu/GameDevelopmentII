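; BP_Gas is a gas trap that repeatedly damages the player while its mesh is overlapped.
; BeginPlay caches the player pawn as BP_ThirdPersonCharacterLabwork3, and the construction script applies the gas material.
; Mesh overlap events toggle a StillInside flag without checking which actor overlaps.
; Tick reads that flag and calls the player's DamageFunction through a DoOnce that resets after a one-second delay.
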(event `self.ReceiveBeginPlay`
  (bind _asbp_third_person_character_labwork_3 (cast `/Game/Classes/LabWork3/BP_ThirdPersonCharacterLabwork3` (`GameplayStatics.GetPlayerPawn` 0)))
  (set `self.Player` _asbp_third_person_character_labwork_3))

(event `self.ReceiveTick`
  (params (DeltaSeconds :type "Float (single-precision)"))
  (if (`self.stillInside`)
    (`/Engine/EditorBlueprintResources/StandardMacros.DoOnce` false :!label _label
      (:`Completed`
        (`/Game/Classes/LabWork3/BP_ThirdPersonCharacterLabwork3.DamageFunction` (`self.Player`))
        (`KismetSystemLibrary.Delay` 1.0)
        (goto _label :!via `Reset`)))))

(event `self.StaticMesh.OnComponentBeginOverlap`
  (params (OverlappedComponent :type "PrimitiveComponent Object Reference") (OtherActor :type "Actor Object Reference") (OtherComp :type "PrimitiveComponent Object Reference") (OtherBodyIndex :type Integer) (bFromSweep :type Boolean) (SweepResult :type "HitResult Structure (by ref)"))
  (set `self.stillInside` true))

(event `self.StaticMesh.OnComponentEndOverlap`
  (params (OverlappedComponent :type "PrimitiveComponent Object Reference") (OtherActor :type "Actor Object Reference") (OtherComp :type "PrimitiveComponent Object Reference") (OtherBodyIndex :type Integer))
  (set `self.stillInside` false))

(fn `UserConstructionScript`
  (`PrimitiveComponent.SetMaterial` (`self.StaticMesh`) 0 "/Game/Classes/Labwork4andMidterm/M/M_GasMaterial.M_GasMaterial"))